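; BP_SnakeElement is a segment of a snake that can be turned into the snake's head.
; On BeginPlay it runs the parent logic, stores a static mesh in Vertebra and binds the mesh component's overlap event to a debug "Hello" print.
; The SetSnakeHead event hides the cylinder, swaps the mesh material and reveals the two eyes and tongue.
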(event `self.ReceiveBeginPlay`
  (`parent.ReceiveBeginPlay`)
  (set `self.vertebra` (`self.StaticMesh`))
  (add `PrimitiveComponent.OnComponentBeginOverlap` (`self.MeshComponent`) (delegate `OnComponentBeginOverlap_Event_0`)))

(event `self.ReceiveActorBeginOverlap`
  (params (OtherActor :type "Actor Object Reference")))

(event `OnComponentBeginOverlap_Event_0`
  (params (OverlappedComponent :type "PrimitiveComponent Object Reference") (OtherActor :type "Actor Object Reference") (OtherComp :type "PrimitiveComponent Object Reference") (OtherBodyIndex :type Integer) (bFromSweep :type Boolean) (SweepResult :type "HitResult Structure (by ref)"))
  (`KismetSystemLibrary.PrintString` "Hello"))

(event `self.SetSnakeHead`
  (`SceneComponent.SetVisibility` (`self.Cylinder`) false false)
  (`PrimitiveComponent.SetMaterial` (`self.MeshComponent`) 0 "/Engine/EngineMaterials/DefaultDecalMaterial.DefaultDecalMaterial")
  (`SceneComponent.SetVisibility` (`self.eye1`) true false)
  (`SceneComponent.SetVisibility` (`self.eye2`) true false)
  (`SceneComponent.SetVisibility` (`self.lang`) true false))

(fn `UserConstructionScript`)